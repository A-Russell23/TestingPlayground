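; AI character Blueprint that keeps an attached health bar widget in sync with the character's health attribute.
; On BeginPlay it sets the bar from current health, then listens with a WaitForAttributeChanged async task for every later change.
; UpdateHealthBar casts the widget component's object to TargetDummyHealthBarWidget and writes health as a fraction of max health.
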(event `self.ReceiveBeginPlay`
  (`self.UpdateHealthBar` (`self.GetHealth`))
  (bind (_asynctaskproxy _attribute _newvalue) (`AbilityAsync_WaitAttributeChanged.WaitForAttributeChanged` null (struct :`AttributeName` "Health" :`Attribute` "/Script/TPProj.CharacterAttributeSetBase:Health" :`AttributeOwner` "Class'\"/Script/TPProj.CharacterAttributeSetBase\"'"))
    (:`Changed`
      (`self.UpdateHealthBar` _newvalue))))

(fn `UpdateHealthBar`
  (params (Health :type "Float (double-precision)"))
  (bind _astarget_dummy_health_bar_widget (cast `/Game/MyAssets/TargetDummyHealthBarWidget` (`WidgetComponent.GetUserWidgetObject` (`self.HealthBar`))))
  (set `/Game/MyAssets/TargetDummyHealthBarWidget.Health` (/ Health (`self.GetMaxHealth`)) _astarget_dummy_health_bar_widget)
  (return))

(fn `UserConstructionScript`)