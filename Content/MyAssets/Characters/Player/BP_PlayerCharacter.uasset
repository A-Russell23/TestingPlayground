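; Player character Blueprint that ties Gameplay Ability System attributes to the HUD, death and respawn.
; BeginPlay saves the spawn transform to BP_ThirdPersonGameMode, waits briefly for possession, then creates the HUD and applies a mana regen GameplayEffect.
; Tick polls health on DemoPlayerState and calls Die at zero, a stopgap for an attribute-change listener.
; When destroyed, the character asks the game mode to respawn the player.
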(event `RegenMana`
  (`AbilitySystemComponent.BP_ApplyGameplayEffectToSelf` :`self` (`AbilitySystemBlueprintLibrary.GetAbilitySystemComponent` self) :`GameplayEffectClass` "/Game/MyAssets/Effects/GE_ManaRegen.GE_ManaRegen_C"))

(event `self.ReceiveBeginPlay`
  (bind _asbp_third_person_game_mode (cast `/Game/BP_ThirdPersonGameMode` (`GameplayStatics.GetGameMode`)))
  (set `/Game/BP_ThirdPersonGameMode.Respawn Transform` (`self.GetTransform`) _asbp_third_person_game_mode)
  ;[1 1 1] Wait for posses
  (`KismetSystemLibrary.Delay` 0.2)
  ;[1 1 1] Set up HUD
  (bind _returnvalue (`|CreateWidget` "/Game/MyAssets/HUDWidget.HUDWidget_C"))
  (bind _output_get (set `self.HealthBar` _returnvalue))
  (`UserWidget.AddToViewport` _output_get 0)
  (`self.RegenMana`))

(event `self.ReceiveTick`
  (params (DeltaSeconds :type "Float (single-precision)"))
  (bind _asdemo_player_state (cast `DemoPlayerState` (`self.PlayerState`)))
  ;[1 1 1] TODO - use wait for attribute changed
  (if (<= (`DemoPlayerState.GetHealth` _asdemo_player_state) 0.0)
    (`self.Die`)))

(event `self.ReceiveDestroyed`
  (bind _asbp_third_person_game_mode (cast `/Game/BP_ThirdPersonGameMode` (`GameplayStatics.GetGameMode`)))
  (`/Game/BP_ThirdPersonGameMode.Player Respawn` _asbp_third_person_game_mode self))

(fn `UserConstructionScript`)