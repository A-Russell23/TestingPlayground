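; Gameplay ability for the fire spell that launches a BP_FireProjectile from the player character's ProjectileSpawnLocation.
; On activation it builds GE_Ablaze (tagged SetByCaller) and GE_Explode specs and hands them to the projectile as its ongoing and immediate effects.
; The owning actor is the DemoPlayerState, whose pawn supplies the transform and instigator.
; CommitAbility runs only after the spawn, and failed casts never reach EndAbility.
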(event `self.K2_ActivateAbility`
  (bind _returnvalue (`AbilitySystemBlueprintLibrary.AssignTagSetByCallerMagnitude` (`self.MakeOutgoingGameplayEffectSpec` "/Game/MyAssets/Effects/GE_Ablaze.GE_Ablaze_C") (struct :`TagName` "State.Debuff.Ablaze")))
  (bind _asdemo_player_state (cast `DemoPlayerState` (`self.GetOwningActorFromActorInfo`))
    (:`then`
      (bind _returnvalue_2 (`PlayerState.GetPawn` _asdemo_player_state))
      (bind _asbp_player_character (cast `/Game/MyAssets/Characters/Player/BP_PlayerCharacter` _returnvalue_2))
      (`|SpawnActorFromClass` "/Game/MyAssets/Abilities/FireSpell/BP_FireProjectile.BP_FireProjectile_C" (`SceneComponent.K2_GetComponentToWorld` (`/Game/MyAssets/Characters/Player/BP_PlayerCharacter.ProjectileSpawnLocation` _asbp_player_character)) "Undefined" "OverrideRootScale" null _returnvalue (`self.MakeOutgoingGameplayEffectSpec` "/Game/MyAssets/Effects/GE_Explode.GE_Explode_C") _returnvalue_2)
      (`self.K2_CommitAbility`)
      (`self.K2_EndAbility`))
    (:`CastFailed`
      (`KismetSystemLibrary.PrintString` "Failed"))))

(event `self.K2_OnEndAbility`
  (params (bWasCancelled :type Boolean)))