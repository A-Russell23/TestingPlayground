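; Gameplay ability for the water spell, which fires a BP_WaterProjectile carrying Wet and Heal gameplay effects.
; On activation it builds both effect specs, tagging Wet with a SetByCaller magnitude, and passes them to the projectile as ongoing and immediate effects.
; The projectile spawns at the player character's ProjectileSpawnLocation, found through the owning PlayerState's pawn.
; CommitAbility runs only after the spawn, then the ability ends.
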(event `self.K2_ActivateAbility`
  (`KismetSystemLibrary.PrintString` "Ability 2")
  (bind _returnvalue (`AbilitySystemBlueprintLibrary.AssignTagSetByCallerMagnitude` (`self.MakeOutgoingGameplayEffectSpec` "/Game/MyAssets/Effects/GE_Wet.GE_Wet_C") (struct :`TagName` "State.Buff.Wet")))
  (bind _asdemo_player_state (cast `DemoPlayerState` (`self.GetOwningActorFromActorInfo`)))
  (bind _returnvalue_2 (`PlayerState.GetPawn` _asdemo_player_state))
  (bind _asbp_player_character (cast `/Game/MyAssets/Characters/Player/BP_PlayerCharacter` _returnvalue_2))
  (`|SpawnActorFromClass` "/Game/MyAssets/Abilities/WaterSpell/BP_WaterProjectile.BP_WaterProjectile_C" (`SceneComponent.K2_GetComponentToWorld` (`/Game/MyAssets/Characters/Player/BP_PlayerCharacter.ProjectileSpawnLocation` _asbp_player_character)) "Undefined" "OverrideRootScale" null _returnvalue (`self.MakeOutgoingGameplayEffectSpec` "/Game/MyAssets/Abilities/WaterSpell/GE_Heal.GE_Heal_C") _returnvalue_2)
  (`self.K2_CommitAbility`)
  (`self.K2_EndAbility`))

(event `self.K2_OnEndAbility`
  (params (bWasCancelled :type Boolean)))