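; Fire sphere effect that sets overlapping demo characters ablaze through the Gameplay Ability System and catches fire itself.
; SetOnFire applies OnPickupEffect as the burn, using the State.Debuff.Ablaze tag to skip targets already burning.
; Once the sphere ignites, it waits briefly, then passes the effect to overlapping BP_FireSphere actors.
; An explode dispatcher bound at BeginPlay strips Ablaze effects from overlapping fire spheres.
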(event `self.ReceiveActorBeginOverlap`
  (params (OtherActor :type "Actor Object Reference"))
  (for _ (`PrimitiveComponent.GetOverlappingActors` (`self.Box`) null)
    (bind _asdemo_character_base (cast `DemoCharacterBase` OtherActor))
    (`self.SetOnFire` (`AbilitySystemBlueprintLibrary.GetAbilitySystemComponent` _asdemo_character_base))))

(event `self.ReceiveBeginPlay`
  (add `self.ExploseDispatch` (delegate `Explode`)))

(event `SetOnFire`
  (params (ASC :type "AbilitySystemComponent Object Reference"))
  (bind _abilitysystem (`self.AbilitySystem`))
  (bind _returnvalue (`AbilitySystemComponent.MakeOutgoingSpec` ASC (`self.OnPickupEffect`) 0.0 (`AbilitySystemComponent.MakeEffectContext` ASC)))
  (if (`KismetSystemLibrary.IsValid` ASC)
    (if (not (>= (`AbilitySystemComponent.GetGameplayTagCount` ASC (struct :`TagName` "State.Debuff.Ablaze")) 1))
      (`AbilitySystemComponent.BP_ApplyGameplayEffectSpecToSelf` ASC _returnvalue)
      (if (not (>= (`AbilitySystemComponent.GetGameplayTagCount` _abilitysystem (struct :`TagName` "State.Debuff.Ablaze")) 1))
        (`AbilitySystemComponent.BP_ApplyGameplayEffectSpecToSelf` _abilitysystem _returnvalue)
        (`KismetSystemLibrary.Delay` 1.0)
        (for _array_element (`self.GetOverlappingActors` "BP_FireSphere_C")
          (bind _returnvalue_2 (`AbilitySystemBlueprintLibrary.GetAbilitySystemComponent` _array_element))
          (if (not (>= (`AbilitySystemComponent.GetGameplayTagCount` _returnvalue_2 (struct :`TagName` "State.Debuff.Ablaze")) 1))
            (`self.SetOnFire` _returnvalue_2)))))))

(event `Explode`
  (for _array_element (`self.GetOverlappingActors` "BP_FireSphere_C")
    (`AbilitySystemComponent.RemoveActiveEffectsWithGrantedTags` (`AbilitySystemBlueprintLibrary.GetAbilitySystemComponent` _array_element) (struct :`GameplayTags` (struct :`(TagName` "State.Debuff.Ablaze"))))))

(fn `UserConstructionScript`)