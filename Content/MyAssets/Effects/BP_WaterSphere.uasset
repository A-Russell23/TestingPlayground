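; BP_WaterSphere is an effect actor that applies a Gameplay Ability System effect to characters that overlap it.
; ActorBeginOverlap casts the other actor to DemoCharacterBase, then applies OnPickupEffect at level zero to that character's own ability system component.
; The actor stays in place afterward, and a loop over the Box's overlapping actors is left unconnected.
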(event `self.ReceiveActorBeginOverlap`
  (params (OtherActor :type "Actor Object Reference"))
  (bind _asdemo_character_base (cast `DemoCharacterBase` OtherActor))
  (bind _returnvalue (`AbilitySystemBlueprintLibrary.GetAbilitySystemComponent` _asdemo_character_base))
  (if (`KismetSystemLibrary.IsValid` _returnvalue)
    (`AbilitySystemComponent.BP_ApplyGameplayEffectSpecToSelf` _returnvalue (`AbilitySystemComponent.MakeOutgoingSpec` _returnvalue (`self.OnPickupEffect`) 0.0 (`AbilitySystemComponent.MakeEffectContext` _returnvalue)))))

(fn `UserConstructionScript`)